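; Game mode for a timed statue-collection game, tracking score, player level, countdown and game-over state.
; StartGame resets the run on BeginPlay or restart and starts a looping Clock timer that flags game over at zero.
; Statue pickups play a sound and add level-scaled score, periodically granting bonus time and a capped level increase.
; AddTime trades score for extra seconds.
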(event Custom|RestartGame1
  (Utilities|StartGame))

(event Custom|Clock
  (Math|Integer|DecrementInt (Variables|Default|GetTime)
    (:%20%20
      (if (== (Variables|Default|GetTime) 0)
        (Variables|Default|SetGameOver true)
        (Utilities|Time|ClearTimerbyFunctionName 0 "Clock")))))

(event EventBeginPlay
  (Utilities|StartGame))

(fn ConstructionScript)

(fn StatueCollected
  (AddComponent|AddAudioComponent false) ; Plays The Collect SFX
  (Variables|Default|SetScore (+ (Variables|Default|GetScore) (* (Variables|Default|GetPlayer_Level) 10)))
  (bind _output_get (Variables|Default|SetStatueCount (+ (Variables|Default|GetStatueCount) 1)))
  (if (== (Math|Integer|%(Integer) _output_get 5) 0)
    (Variables|Default|SetTime (+ (Variables|Default|GetTime) 15))
    (Variables|Default|SetPlayer_Level (Math|Integer|Min(Integer) (+ (Variables|Default|GetPlayer_Level) 1) 5))))

(fn AddTime
  (if (> (Variables|Default|GetScore) 10)
    (Variables|Default|SetTime (+ (Variables|Default|GetTime) 10))
    (Variables|Default|SetScore (- (Variables|Default|GetScore) 10))))