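; BP_Statue is a collectible that jumps around the level until the player touches it.
; InitStatue teleports it to a random ground-plane position and re-arms a timer on itself, with the delay shrinking as the game mode's player level rises.
; When the player pawn overlaps it before game over, it reports the collection to BP_GameMode_Lab4, destroys itself and spawns an actor at the game mode's transform.
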(event EventBeginPlay
  (bind _asbp_game_mode_lab_4 (Utilities|Casting|CastToBP_GameMode_Lab4 (Game|GetGameMode)))
  (Variables|Default|SetAs%20BP%20Game%20Mode%20Lab%204 _asbp_game_mode_lab_4)
  (CallFunction|InitStatue))

(event Collision|EventActorBeginOverlap
  (params (OtherActor :type Actor%20Object%20Reference))
  (if (and (== OtherActor (Game|Player|GetPlayerPawn 0)) (not (Variables|/Game/2202784/BP_GameMode_Lab4.BP_GameMode_Lab4_C|GetGameOver (Variables|Default|GetAs%20BP%20Game%20Mode%20Lab%204))))
    (Default|StatueCollected (Variables|Default|GetAs%20BP%20Game%20Mode%20Lab%204))
    (Actor|DestroyActor)
    (Game|SpawnActorfromClass "BP_Statue_C" (Transformation|GetActorTransform (Variables|Default|GetAs%20BP%20Game%20Mode%20Lab%204)) "Undefined" "MultiplyWithRoot" 0 0)))

(fn ConstructionScript)

(fn InitStatue
  (Transformation|Teleport (Math|Vector|MakeVector (Math|Random|RandomFloatinRange 0.0 2e+03) (Math|Random|RandomFloatinRange 2e+02 2e+03) 0.0) "0, 0, 0")
  (Utilities|Time|SetTimerbyFunctionName 0 "InitStatue" (Math|Conversions|ToFloat(Integer) (- 6 (Variables|/Game/2202784/BP_GameMode_Lab4.BP_GameMode_Lab4_C|GetPlayer_Level (Variables|Default|GetAs%20BP%20Game%20Mode%20Lab%204))))))