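; HUD Blueprint for Lab 4 that draws the game's status text directly on screen.
; On BeginPlay it casts and caches the Lab 4 game mode, then each DrawHUD call reads that reference to show time, score, player level and statue count along the top.
; When the game mode's GameOver flag is set, it also draws a game-over message and a restart prompt, though restart input is not handled here.
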(event EventBeginPlay
  (bind _asbp_game_mode_lab_4 (Utilities|Casting|CastToBP_GameMode_Lab4 (Game|GetGameMode)))
  (Variables|Default|SetAs%20BP%20Game%20Mode%20Lab%204 _asbp_game_mode_lab_4))

(event EventDrawHUD
  (params (SizeX :type Integer) (SizeY :type Integer))
  (bind _as_bp_game_mode_lab_4 (Variables|Default|GetAs%20BP%20Game%20Mode%20Lab%204))
  (HUD|DrawText (Utilities|String|BuildString(Integer) "Time:" "" (Variables|/Game/2202784/BP_GameMode_Lab4.BP_GameMode_Lab4_C|GetTime _as_bp_game_mode_lab_4)) "(R=0.000000,G=0.000000,B=0.000000,A=1.000000)" 1e+01 1e+01 0 3.0 false)
  (HUD|DrawText (Utilities|String|BuildString(Integer) "Score:" "" (Variables|/Game/2202784/BP_GameMode_Lab4.BP_GameMode_Lab4_C|GetScore _as_bp_game_mode_lab_4)) "(R=0.000000,G=0.000000,B=0.000000,A=1.000000)" 2e+02 1e+01 0 3.0 false)
  (HUD|DrawText (Utilities|String|BuildString(Integer) "Player Level:" "" (Variables|/Game/2202784/BP_GameMode_Lab4.BP_GameMode_Lab4_C|GetPlayer_Level _as_bp_game_mode_lab_4)) "(R=0.000000,G=0.000000,B=0.000000,A=1.000000)" 4e+02 1e+01 0 3.0 false)
  (HUD|DrawText (Utilities|String|BuildString(Integer) "Statue Count :" "" (Variables|/Game/2202784/BP_GameMode_Lab4.BP_GameMode_Lab4_C|GetStatueCount _as_bp_game_mode_lab_4)) "(R=0.000000,G=0.000000,B=0.000000,A=1.000000)" 8.5e+02 1e+01 0 3.0 false)
  (if (Variables|/Game/2202784/BP_GameMode_Lab4.BP_GameMode_Lab4_C|GetGameOver (Variables|Default|GetAs%20BP%20Game%20Mode%20Lab%204))
    (HUD|DrawText "GAME OVER" "(R=1.000000,G=0.000000,B=0.382729,A=1.000000)" 4e+02 2e+02 0 1.0 false)
    (HUD|DrawText "PRESS ENTER TO RESTART" "(R=0.058333,G=0.000000,B=0.000000,A=1.000000)" 4e+02 4.5e+02 0 1.0 false)))

(fn ConstructionScript)